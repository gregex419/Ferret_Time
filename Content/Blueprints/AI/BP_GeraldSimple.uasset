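; Simple AI for Gerald, an NPC racing the player for his phone, keys and wallet, triggering a loss once he has all three.
; After a head start, chained AIMoveTo events, not a Behavior Tree, alternate patrol with random roaming and chance-based item searches at set points.
; AI Perception triggers chasing players carrying key items; catching one forces a drop and teleports them to PlayerStart.
; Overlaps collect items; Tick checks the loss.
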(event OnComponentBeginOverlap(Pickup/Tag)
  (params (OverlappedComponent :type Primitive%20Component%20Object%20Reference) (OtherActor :type Actor%20Object%20Reference) (OtherComp :type Primitive%20Component%20Object%20Reference) (OtherBodyIndex :type Integer) (bFromSweep :type Boolean) (SweepResult :type Hit%20Result%20Structure%20%28by%20ref%29))
  ;[0 1 1] Key Items Pickups
  ;;[0 1 1] Check if Gerald picked up a key item
  (Utilities|FlowControl|Sequence
    (:then_0
      (bind _asbp_phone (Utilities|Casting|CastToBP_Phone OtherActor))
      (Actor|DestroyActor _asbp_phone)
      (Variables|Default|SetGeraldPhone true)
      (Default|CallGeraldHasPhone))
    (:then_1
      (bind _asbp_keys (Utilities|Casting|CastToBP_Keys OtherActor))
      (Actor|DestroyActor _asbp_keys)
      (Variables|Default|SetGeraldKeys true)
      (Default|CallGeraldHasKeys))
    (:then_2
      (bind _asbp_wallet (Utilities|Casting|CastToBP_Wallet OtherActor))
      (Actor|DestroyActor _asbp_wallet)
      (Variables|Default|SetGeraldWallet true)
      (Default|CallGeraldHasWallet))))

(event OnTargetPerceptionUpdated(AIPerception)
  (params (Actor :type Actor%20Object%20Reference) (Stimulus :type AI%20Stimulus%20Structure))
  ;[1 1 1] AI Behavior Setup
  ;;[1 0 1] What happens when the player is seen (Figure out entering and exiting the pawn sensing... Specifically Exiting)
  (bind _asbp_animal_character (Utilities|Casting|CastToBP_AnimalCharacter Actor))
  ;;;[1 0 1] True = Player is seen
  ;;; Fales = Lost Sight of Player
  (if (.bSuccessfullySensed (Utilities|Struct|BreakAIStimulus Stimulus))
    (Variables|/Game/Blueprints/GameBase/BP_AnimalCharacter.BP_AnimalCharacter_C|SetIsSeen _asbp_animal_character true)
    (if (Variables|/Game/Blueprints/GameBase/BP_AnimalCharacter.BP_AnimalCharacter_C|GetHasKeyItem _asbp_animal_character)
      (CallFunction|ChasePlayer)
      (else
        (CallFunction|Patrol :!label _label)))
    (else
      (CallFunction|GotoLastLocation)
      (Utilities|FlowControl|Delay 5.0)
      (goto _label))))

(event Custom|Roam%20Around
  ;[1 1 1] AI Behavior Setup
  ;;[0 1 0] Basic Roaming Setup
  (AI|AIMoveTo self (.RandomLocation (Class|NavigationSystemV1|GetRandomPointinNavigableRadius (Transformation|GetActorLocation) 5e+02 (Variables|Default|GetNavMeshArea) "/Script/AIModule.NavFilter_AIControllerDefault")) 0 5.0 false
    (:OnSuccess
      (Utilities|FlowControl|Delay 1.0) ; Wait time between points
      (Variables|Default|SetRoamCounter (- (Variables|Default|GetRoamCounter) 1))
      (if (<= (Variables|Default|GetRoamCounter) 0)
        ;;[0 1 1] Pre-Item Check
        (Utilities|FlowControl|Sequence
          (:then_0
            (if (== (Variables|Default|GetCurrentPatrolPointsIndex) 4)
              (CallFunction|ItemSearchWallet)
              (else
                (CallFunction|Patrol :!label _label))))
          (:then_1
            (if (== (Variables|Default|GetCurrentPatrolPointsIndex) 8)
              (CallFunction|ItemSearchPhone)
              (else
                (goto _label))))
          (:then_2
            (if (== (Variables|Default|GetCurrentPatrolPointsIndex) 12)
              (CallFunction|ItemSearchKeys)
              (else
                (goto _label)))))
        (else
          (CallFunction|RoamAround))))))

(event Custom|Chase%20Player
  ;[1 1 1] AI Behavior Setup
  ;;[1 0 0] Basic Player Chase
  (AI|AIMoveTo self "0, 0, 0" (Game|GetPlayerCharacter 0) 0.01 false
    (:OnSuccess
      (bind _asbp_animal_character (Utilities|Casting|CastToBP_AnimalCharacter (Game|Player|GetPlayerPawn 0)))
      (bind _outactors (Actor|GetAllActorsOfClass "/Script/Engine.PlayerStart"))
      (Default|DropObject _asbp_animal_character)
      (Transformation|Teleport _asbp_animal_character (Transformation|GetActorLocation (Utilities|Array|Get(acopy) _outactors)) "0, 0, 0"))))

(event Custom|GoToLastLocation
  ;[1 1 1] AI Behavior Setup
  ;;[1 0 1] What happens when the player is seen (Figure out entering and exiting the pawn sensing... Specifically Exiting)
  (AI|Navigation|SimpleMovetoLocation (Pawn|GetController self) (.StimulusLocation (Utilities|Struct|BreakAIStimulus (stale OnTargetPerceptionUpdated(AIPerception) Stimulus)))))

(event Custom|ItemSearchPhone
  ;[0 1 1] Key Items Pickups
  ;;[0 1 1] Can you check for the items/Will you stay in that room?
  (if (== (Math|Random|RandomIntegerinRange 1 3) 1)
    (CallFunction|GotoPhone)
    (elif (== (Math|Random|RandomIntegerinRange 1 2) 1)
      (CallFunction|Patrol)
      (else
        (CallFunction|RoamAround)))))

(event Custom|You're%20a%20Lose%20:%28
  ;[1 1 1] Losing Condition
  (if (Math|Boolean|ANDBoolean (Variables|Default|GetGeraldPhone) (Variables|Default|GetGeraldKeys) (Variables|Default|GetGeraldWallet))
    (Default|CallYouLose)))

(event Custom|Head%20Start
  ;[1 1 1] AI Behavior Setup
  ;;[1 1 0] Checks to see if head start is complete
  ;;;[1 0.5 0] Head Start Delay
  (Utilities|FlowControl|Delay (Variables|Default|GetHeadStartCountdown))
  (CallFunction|Patrol))

(event Custom|AI%20Switches
  ;[1 1 1] Manual Control System (Make AIState public to debug)
  (switch Utilities|FlowControl|Switch|SwitchonEnum_AI_State (Variables|Default|GetAIState)
    (:NewEnumerator1
      (CallFunction|RoamAround))
    (:NewEnumerator2
      (CallFunction|ChasePlayer))
    (:NewEnumerator3
      (CallFunction|Patrol))))

(event Custom|GoToWallet
  (bind _walletlocation (Variables|Default|GetWalletLocation))
  ;[0 1 1] Key Items Pickups
  ;;[0 1 1] Move to Pickup Wallet
  ;;;[0 1 1] Moves the AI to its destination
  (AI|AIMoveTo self "0, 0, 0" (Utilities|Array|Get(acopy) _walletlocation) 0.1 false ; Acceptance Radius = How Close To Target
    (:OnSuccess
      ;;;[0 1 1] Moves the AI to its destination
      (AI|AIMoveTo self "0, 0, 0" (Utilities|Array|Get(acopy) _walletlocation 1) 0.1 false ; Acceptance Radius = How Close To Target
        (:OnSuccess
          (Utilities|FlowControl|Delay 3.0)
          (CallFunction|Patrol))))))

(event Custom|Patrol
  ;[1 1 1] AI Behavior Setup
  ;;[0 0 1] AI Patrol
  ;;;[0 0 1] This sends the AI to a point right before the main point. Use the first set of points to have the character facing the right direction when they get to the inportant target point.
  ;;;;[0 0 1] Event Patrol
  ;;;;[0 0 1] Moves the AI to its destination
  (AI|AIMoveTo self "0, 0, 0" (Utilities|Array|Get(acopy) (Variables|Default|GetPatrolPoints) (Variables|Default|GetCurrentPatrolPointsIndex)) 5.0 false ; Acceptance Radius = How Close To Target
    (:OnSuccess
      ;;;;[0 0 1] Returns if you have reached the end of the patrol points or not...
      (if (>= (Variables|Default|GetCurrentPatrolPointsIndex) (- (Utilities|Array|Length (Variables|Default|GetPatrolPoints)) 1))
        ;;;;[0 0 1] Resets the patrol points to 0
        (Variables|Default|SetCurrentPatrolPointsIndex 0)
        (else
          ;;;;[0 0 1] Incriments to the next patrol point
          (Math|Integer|IncrementInt (Variables|Default|GetCurrentPatrolPointsIndex)
            (:%20%20
              _))))
      ;;;[0 0 1] Are we at the main Patrol Point?
      (if (<= (Variables|Default|GetPatrolCountdown) 1)
        ;;;[1 0.5 0] Reset non-main patrol points (should be same as hard coded number)
        (Variables|Default|SetPatrolCountdown 4)
        ;;;[1 0.5 0] Time Between Targets
        (Utilities|FlowControl|Delay 1.0)
        ;;[0 1 0] Roam Setup
        (Variables|Default|SetRoamCounter (Math|Random|RandomIntegerinRange 2 5))
        (CallFunction|RoamAround)
        (else
          ;;;[0 0 1] Decrease number of non-main patrol points to patrol
          (Variables|Default|SetPatrolCountdown (- (Variables|Default|GetPatrolCountdown) 1))
          ;;;[0 0 1] Repeat Patrol
          (CallFunction|Patrol))))))

(event Custom|GoToPhone
  (bind _phonelocation (Variables|Default|GetPhoneLocation))
  ;[0 1 1] Key Items Pickups
  ;;[0 1 1] Move to Pickup Phone
  ;;;[0 1 1] Moves the AI to its destination
  (AI|AIMoveTo self "0, 0, 0" (Utilities|Array|Get(acopy) _phonelocation) 0.1 false ; Acceptance Radius = How Close To Target
    (:OnSuccess
      ;;;[0 1 1] Moves the AI to its destination
      (AI|AIMoveTo self "0, 0, 0" (Utilities|Array|Get(acopy) _phonelocation 1) 0.1 false ; Acceptance Radius = How Close To Target
        (:then
          (Utilities|FlowControl|Delay 3.0)
          (CallFunction|Patrol))))))

(event Custom|ItemSearchKeys
  ;[0 1 1] Key Items Pickups
  ;;[0 1 1] Can you check for the items/Will you stay in that room?
  (if (== (Math|Random|RandomIntegerinRange 1 3) 1)
    (CallFunction|GotoKeys)
    (elif (== (Math|Random|RandomIntegerinRange 1 2) 1)
      (CallFunction|Patrol)
      (else
        (CallFunction|RoamAround)))))

(event Custom|GoToKeys
  (bind _keyslocation (Variables|Default|GetKeysLocation))
  ;[0 1 1] Key Items Pickups
  ;;[0 1 1] Move to Pickup Keys
  ;;;[0 1 1] Moves the AI to its destination
  (AI|AIMoveTo self "0, 0, 0" (Utilities|Array|Get(acopy) _keyslocation) 0.1 false ; Acceptance Radius = How Close To Target
    (:OnSuccess
      ;;;[0 1 1] Moves the AI to its destination
      (AI|AIMoveTo self "0, 0, 0" (Utilities|Array|Get(acopy) _keyslocation 1) 0.1 false ; Acceptance Radius = How Close To Target
        (:OnSuccess
          (Utilities|FlowControl|Delay 3.0)
          (CallFunction|Patrol))))))

(event Custom|ItemSearchWallet
  ;[0 1 1] Key Items Pickups
  ;;[0 1 1] Can you check for the items/Will you stay in that room?
  (if (== (Math|Random|RandomIntegerinRange 1 3) 1)
    (CallFunction|GotoWallet)
    (elif (== (Math|Random|RandomIntegerinRange 1 2) 1)
      (CallFunction|Patrol)
      (else
        (CallFunction|RoamAround)))))

(event EventBeginPlay
  (CallFunction|HeadStart))

(event EventTick
  (params (DeltaSeconds :type Float%20%28single-precision%29))
  (CallFunction|You'reALose:())

(fn ConstructionScript)