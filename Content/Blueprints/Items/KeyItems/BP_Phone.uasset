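; BP_Phone is a key item Blueprint that controls the HasKeyItem flag on the player's BP_AnimalCharacter.
; Every Tick, it casts player pawn 0 to BP_AnimalCharacter and binds to that character's IsPickedUp and IsDropped dispatchers, rather than binding once in BeginPlay.
; The pickup event sets HasKeyItem to true and the drop event clears it, with no check in this graph on which item was involved.
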(event Custom|ActivateHasKeyItem
  (Variables|/Game/Blueprints/GameBase/BP_AnimalCharacter.BP_AnimalCharacter_C|SetHasKeyItem (stale EventTick _asbp_animal_character) true))

(event Custom|DeactivateHasKeyItem
  (Variables|/Game/Blueprints/GameBase/BP_AnimalCharacter.BP_AnimalCharacter_C|SetHasKeyItem (stale EventTick _asbp_animal_character) false))

(event EventBeginPlay
  (|CallParentFunction))

(event EventTick
  (params (DeltaSeconds :type Float%20%28single-precision%29))
  (bind _asbp_animal_character (Utilities|Casting|CastToBP_AnimalCharacter (Game|Player|GetPlayerPawn 0)))
  (EventDispatchers|BindEventtoIsPickedUp _asbp_animal_character (delegate Custom|ActivateHasKeyItem))
  (EventDispatchers|BindEventtoIsDropped _asbp_animal_character (delegate Custom|DeactivateHasKeyItem)))

(fn ConstructionScript
  (|CallParentFunction))